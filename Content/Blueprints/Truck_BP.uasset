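; Truck actor that drives along its local Y axis in a repeating loop, snapping back to its start point.
; BeginPlay stores the root component's world location, then a looping Delay returns the actor there every three seconds.
; Tick, throttled by a short Delay, adds a swept local offset of random size, so speed varies from step to step.
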(event EventBeginPlay
  (Variables|Default|SetSpawn (Transformation|GetWorldLocation (Variables|Default|GetDefaultSceneRoot)))
  (Utilities|FlowControl|Delay 3.0 :!label _label)
  (Utilities|Time|ClearTimerbyFunctionName 0 "")
  (Transformation|SetActorLocation (Variables|Default|GetSpawn) false false)
  (goto _label))

(event Collision|EventActorBeginOverlap
  (params (OtherActor :type Actor%20Object%20Reference)))

(event EventTick
  (params (DeltaSeconds :type Float%20%28single-precision%29))
  (Utilities|FlowControl|Delay 0.03)
  (Transformation|AddActorLocalOffset (Math|Vector|MakeVector 0.0 (Math|Random|RandomFloatinRange 1e+01 2e+01) 0.0) true false))

(fn ConstructionScript)