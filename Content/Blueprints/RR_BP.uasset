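; RR_BP is a construction-script Blueprint that builds a repeating row of static mesh segments along its local Y axis.
; For each of HowManyRR iterations it adds two static mesh components at Counter times RRWidth, the second one unit lower in Z.
; A separately incremented Counter drives the spacing instead of the loop index, and the event graph holds no active logic.
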(event EventBeginPlay)

(event Collision|EventActorBeginOverlap
  (params (OtherActor :type Actor%20Object%20Reference)))

(event EventTick
  (params (DeltaSeconds :type Float%20%28single-precision%29)))

(fn ConstructionScript
  (for _index (range 1 (Variables|Default|GetHowManyRR))
    (AddComponent|AddStaticMeshComponent false (Math|Conversions|ToTransform(Vector) (Math|Vector|MakeVector 0.0 (* (Variables|Default|Getcounter) (Variables|Default|GetRRWidth)) 0.0)))
    (AddComponent|AddStaticMeshComponent false (Math|Conversions|ToTransform(Vector) (Math|Vector|MakeVector 0.0 (* (Variables|Default|Getcounter) (Variables|Default|GetRRWidth)) -1.0)))
    (Variables|Default|Setcounter (+ (Variables|Default|Getcounter) 1))))