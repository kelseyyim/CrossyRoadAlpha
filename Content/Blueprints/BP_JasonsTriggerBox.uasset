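; BP_JasonsTriggerBox is a self-replacing trigger that generates more terrain when an actor, meant to be the chicken, overlaps it.
; On overlap it spawns a new copy of itself, offset along its local X by Counter times GrassWidth.
; A loop then lays grass tiles at increasing offsets, each paired with a road at a random negative X and fixed side offset.
; The box then destroys itself, leaving its copy as the next trigger.
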(event Collision|EventActorBeginOverlap
  (params (OtherActor :type Actor%20Object%20Reference))
  (Game|SpawnActorfromClass "BP_JasonsTriggerBox_C" (Math|Conversions|ToTransform(Vector) (Math|Transform|TransformLocation (Transformation|GetActorTransform) (Math|Vector|MakeVector (* (Variables|Default|Getcounter) (Variables|Default|GetGrassWidth)) 0.0 0.0))) "Undefined" 0 2.8e+02 0)
  (for _index (range 1 (Variables|Default|GetMaxIndex))
    (Game|SpawnActorfromClass "/Game/Materials/GrassBP.GrassBP_C" (Math|Conversions|ToTransform(Vector) (Math|Transform|TransformLocation (Transformation|GetActorTransform) (Math|Vector|MakeVector (* (Variables|Default|Getcounter) (Variables|Default|GetGrassWidth)) 0.0 -1.2e+02))) "Undefined" 0 0)
    (Variables|Default|Setcounter (+ (Variables|Default|Getcounter) 1))
    (Game|SpawnActorfromClass "/Game/Blueprints/Road_BP.Road_BP_C" (Math|Conversions|ToTransform(Vector) (Math|Transform|TransformLocation (Transformation|GetActorTransform) (Math|Vector|MakeVector (Math|Random|RandomFloatinRange -1e+03 -9e+01) -1.7e+03 -123.0))) "Undefined" 0 0))
  (Actor|DestroyActor))

(fn ConstructionScript)